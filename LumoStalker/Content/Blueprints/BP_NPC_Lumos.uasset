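; Lumos is a glowing stalker NPC that hides when watched, circles behind the player, then approaches and attacks.
; Tick computes view dot products and distances, then fires a dispatcher that ChangeState rebinds to one state function: Hide, Sneak, Approach, Retreat, Teleport or Attack.
; States pick transitions from those values and timeouts, moving via AIMoveTo or random teleports after attacks and long stares.
; Point light intensity combines movement, attack build-up and looping flicker.
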(event `self.ReceiveBeginPlay`
  (`self.Event ChangeState` "NewEnumerator0"))

(event `self.ReceiveTick`
  (params (DeltaSeconds :type "Float (single-precision)"))
  ;[1 1 1] Calculate dots and distances
  (set `self.runTime` (+ DeltaSeconds (`self.runTime`)))
  (set `self.deltaTime` DeltaSeconds)
  (bind _dot (`self.Dot To Camera Forward`))
  (set `self.dotToCamForward` _dot)
  (bind _sqrdist (`self.Sqr Dist To Player`))
  (set `self.sqrtDistToPlayer` _sqrdist)
  (bind (_dot_left_right _dot_front_back) (`self.Dot To Player`))
  (set `self.dotPlayerLeftRight` _dot_left_right)
  (set `self.dotPlayerFrontBack` _dot_front_back)
  (`self.Dispatcher UpdateActiveState`)
  ;[0.3281 0.3281 0.3281] Update Light Intensity
  ;;[1 1 1] Add light intensity while moving, gravitate to 0 when stationary
  (if (> (`KismetMathLibrary.VSizeSquared` (`self.GetVelocity`)) 0.0)
    (set `self.currentVelocityIntensity` (+ (`self.currentVelocityIntensity`) (/ (`self.deltaTime`) (`self.timeToMaxIntensity`))))
    (elif (> (`self.currentVelocityIntensity`) 0.0)
      (set `self.currentVelocityIntensity` (- (`self.currentVelocityIntensity`) (`self.deltaTime`)))))
  (set `self.currentVelocityIntensity` (`KismetMathLibrary.FClamp` (`self.currentVelocityIntensity`)))
  (`LightComponent.SetIntensity` (`self.PointLight`) (+ (* (`CurveFloat.GetFloatValue` (`self.LightVelocityIntensity`) (`self.currentVelocityIntensity`)) (`self.maxVelocityIntensity`)) (`self.attackLightIntensity`) (* (`CurveFloat.GetFloatValue` (`self.FlickerCurve`) (mod (`self.runTime`) 2.0)) 50.0))))

(event `Event ChangeState`
  (params (NewState :type "/Game/Blueprints/Data/E_NPC_AIStates_Lumos Enum" :default "NewEnumerator0"))
  ;[1 1 1] State Machine
  (clear `self.Dispatcher UpdateActiveState`)
  (set `self.stateInitialized` false)
  (switch `/Game/Blueprints/Data/E_NPC_AIStates_Lumos` NewState
    (:`NewEnumerator0`
      (add `self.Dispatcher UpdateActiveState` (delegate `Event StateHide`)))
    (:`NewEnumerator1`
      (add `self.Dispatcher UpdateActiveState` (delegate `Event StateSneak`)))
    (:`NewEnumerator2`
      (add `self.Dispatcher UpdateActiveState` (delegate `Event StateApproach`)))
    (:`NewEnumerator3`
      (add `self.Dispatcher UpdateActiveState` (delegate `Event StateRetreat`)))
    (:`NewEnumerator4`
      (add `self.Dispatcher UpdateActiveState` (delegate `Event StateTeleport`)))
    (:`NewEnumerator5`
      (add `self.Dispatcher UpdateActiveState` (delegate `Event StateAttack`)))))

(event `Event StateHide`
  ;[1 1 1] State Machine
  (`self.State Hide`))

(event `Event StateSneak`
  ;[1 1 1] State Machine
  (`self.State Sneak`))

(event `Event StateApproach`
  ;[1 1 1] State Machine
  (`self.State Approach`))

(event `Event StateRetreat`
  ;[1 1 1] State Machine
  (`self.State Retreat`))

(event `Event StateTeleport`
  ;[1 1 1] State Machine
  (`self.State Teleport`))

(event `Event StateAttack`
  ;[1 1 1] State Machine
  (`self.State Attack`))

(event `Event SetDestination`
  (params (Destination :type "Vector Structure"))
  ;[1 1 1] Movement
  (`|AIMoveTo` self Destination null
    (:`then`
      (set `self.isPathfinding` true))
    (:`OnSuccess`
      (set `self.isPathfinding` false :!label _label))
    (:`OnFail`
      (goto _label))))

(event `Event AttackPlayer`
  ;[1 1 1] Send a damage event to player to indicate that they got attacked
  (bind _asbp_first_person_character (cast `/Game/FirstPerson/Blueprints/BP_FirstPersonCharacter` (`GameplayStatics.GetPlayerPawn` 0)))
  (`/Game/FirstPerson/Blueprints/BP_FirstPersonCharacter.Event Damaged` _asbp_first_person_character))

(fn `Dot To Camera Forward`
  (returns (Dot :type "Float (double-precision)"))
  (bind _returnvalue (`GameplayStatics.GetPlayerCameraManager` 0))
  (return (`KismetMathLibrary.Dot_VectorVector` (`KismetMathLibrary.Normal` (- (`self.K2_GetActorLocation` self) (`PlayerCameraManager.GetCameraLocation` _returnvalue))) (`KismetMathLibrary.Normal` (`self.GetActorForwardVector` _returnvalue)))))

(fn `Dot To Player`
  (returns (`Dot Left/Right` :type "Float (double-precision)") (`Dot Front/Back` :type "Float (double-precision)"))
  (bind (_location _rotation) (`Controller.GetPlayerViewPoint` (`GameplayStatics.GetPlayerController` 0)))
  (bind _returnvalue (`KismetMathLibrary.Vector_Normal2D` (- (`self.K2_GetActorLocation`) _location)))
  (return (`KismetMathLibrary.Dot_VectorVector` _returnvalue (`KismetMathLibrary.Vector_Normal2D` (`KismetMathLibrary.GetRightVector` _rotation))) (`KismetMathLibrary.Dot_VectorVector` _returnvalue (`KismetMathLibrary.Vector_Normal2D` (`KismetMathLibrary.GetForwardVector` _rotation)))))

(fn `Sqr Dist To Player`
  (returns (SqrDist :type "Float (double-precision)"))
  (return (`KismetMathLibrary.VSizeSquared` (- (`self.K2_GetActorLocation` self) (`PlayerCameraManager.GetCameraLocation` (`GameplayStatics.GetPlayerCameraManager` 0))))))

(fn `State Approach`
  (if (`self.debugStates`)
    (`KismetSystemLibrary.PrintString` "APPROACH"))
  (`|ExecutionSequence`
    (:`then_0`
      ;[1 1 1] Check for state changes
      (`|ExecutionSequence`
        (:`then_1`
          (if (>= (`self.dotToCamForward`) (`self.dot_ApproachTreshold`))
            (`self.Event ChangeState` "NewEnumerator1")
            (return)))
        (:`then_2`
          (if (<= (`self.sqrtDistToPlayer`) (`self.dist_AttackTreshold`))
            (`self.Event ChangeState` "NewEnumerator5")
            (return)))))
    (:`then_1`
      (if (not (`self.isPathfinding`))
        (`self.Event SetDestination` (+ (`self.K2_GetActorLocation`) (* (`KismetMathLibrary.Vector_Normal2D` (- (`Controller.GetPlayerViewPoint` (`GameplayStatics.GetPlayerController` 0)) (`self.K2_GetActorLocation`))) 100)))
        (return)))))

(fn `State Attack`
  (if (not (`self.stateInitialized`))
    ;[1 1 1] Initialize State
    (set `self.stateInitialized` true)
    (set `self.timeStamp` (`self.runTime`))
    (set `self.attackSuccess` false)
    (set `self.attackLightIntensity` 0.0))
  (if (`self.debugStates`)
    (`KismetSystemLibrary.PrintString` "ATTACK"))
  (`|ExecutionSequence`
    (:`then_0`
      ;[1 1 1] Check for state changes
      (`|ExecutionSequence`
        (:`then_0`
          (if (> (`self.sqrtDistToPlayer`) (`self.dist_AttackTreshold`))
            (`self.Event ChangeState` "NewEnumerator2")
            (set `self.attackLightIntensity` 0.0 :!label _label)
            (return)))
        (:`then_1`
          (if (>= (`self.dotToCamForward`) (`self.dot_ApproachTreshold`))
            (`self.Event ChangeState` "NewEnumerator1")
            (goto _label)))
        (:`then_2`
          (if (`self.attackSuccess`)
            (`self.Event ChangeState` "NewEnumerator4")
            (goto _label)))))
    (:`then_1`
      (if (>= (- (`self.runTime`) (`self.timeStamp`)) (`self.attackTimeout`))
        (`self.Event AttackPlayer`)
        (set `self.attackSuccess` true)
        (else
          ;[1 1 1] Increase light intensity as attack builds up
          (set `self.stateTimer` (- (`self.runTime`) (`self.timeStamp`)))
          (set `self.attackLightIntensity` (* (/ (`self.stateTimer`) (`self.attackTimeout`)) (`self.maxAttackLightIntensity`))))))))

(fn `State Hide`
  (if (not (`self.stateInitialized`))
    ;[1 1 1] Initialize State
    (set `self.stateInitialized` true)
    (set `self.escapeHide` false)
    (set `self.timeStamp` (`self.runTime`)))
  (if (`self.debugStates`)
    (`KismetSystemLibrary.PrintString` "HIDING"))
  (`|ExecutionSequence`
    (:`then_0`
      ;[1 1 1] Check for state changes
      (`|ExecutionSequence`
        (:`then_0`
          (if (< (`self.sqrtDistToPlayer`) (`self.dist_RetreatThreshold`))
            (`self.Event ChangeState` "NewEnumerator3")))
        (:`then_1`
          (if (< (`self.dotToCamForward`) (`self.dot_HideTreshold`))
            (`self.Event ChangeState` "NewEnumerator1")))
        (:`then_2`
          (if (`self.escapeHide`)
            (`self.Event ChangeState` "NewEnumerator4")))))
    (:`then_1`
      ;[1 1 1] Timeout if you stare to long
      (if (>= (- (`self.runTime`) (`self.timeStamp`)) (`self.hideTimeout`))
        (set `self.escapeHide` true)))))

(fn `State Retreat`
  (bind _returnvalue (`self.GetActorRightVector` self))
  (if (not (`self.stateInitialized`))
    ;[1 1 1] Initialize State
    (set `self.stateInitialized` true)
    (set `self.timeStamp` (`self.runTime`)))
  (if (`self.debugStates`)
    (`KismetSystemLibrary.PrintString` "RETREAT"))
  (`|ExecutionSequence`
    (:`then_0`
      ;[1 1 1] Check for state changes
      (if (>= (- (`self.runTime`) (`self.timeStamp`)) (`self.retreatTimeout`))
        (`self.Event ChangeState` "NewEnumerator0")
        (return)))
    (:`then_1`
      ;[1 1 1] Calculate a retreat vector
      (if (not (`self.isPathfinding`))
        (`self.Event SetDestination` (+ (`self.K2_GetActorLocation`) (* (`KismetMathLibrary.Vector_Normal2D` (- (`self.K2_GetActorLocation`) (`Controller.GetPlayerViewPoint` (`GameplayStatics.GetPlayerController` 0)))) 100) (* (select `bool` (`KismetMathLibrary.RandomBool`) :`false` _returnvalue :`true` (* _returnvalue -1)) (`KismetMathLibrary.RandomInteger` 200))))))))

(fn `State Sneak`
  (locals (TargetAngle :type "Float (double-precision)") (RotationStep :type "Float (double-precision)" :default 10.0))
  (if (not (`self.stateInitialized`))
    ;[1 1 1] Initialize State
    (set `self.stateInitialized` true)
    (set `self.distToPlayer` (`KismetMathLibrary.Sqrt` (`self.sqrtDistToPlayer`))))
  (if (`self.debugStates`)
    (`KismetSystemLibrary.PrintString` "SNEAK"))
  (`|ExecutionSequence`
    (:`then_0`
      ;[1 1 1] Check for state changes
      (`|ExecutionSequence`
        (:`then_0`
          (if (>= (`self.dotToCamForward`) (`self.dot_HideTreshold`))
            (`self.Event ChangeState` "NewEnumerator0")
            (return)))
        (:`then_1`
          (if (< (`self.sqrtDistToPlayer`) (`self.dist_RetreatThreshold`))
            (`self.Event ChangeState` "NewEnumerator3")
            (return)))
        (:`then_2`
          (if (< (`self.dotPlayerFrontBack`) (`self.dot_ApproachTreshold`))
            (`self.Event ChangeState` "NewEnumerator2")
            (return)))))
    (:`then_1`
      (if (not (`self.isPathfinding`))
        ;[1 1 1] Decrease distance from player if to far away
        (if (> (`self.distToPlayer`) (`self.dist_SneakPreference`))
          (set `self.distToPlayer` (- (`self.distToPlayer`) 50.0)))
        ;[1 1 1] To the left or right of player forward?
        (bind (_dot_left_right _dot_front_back) (`self.Dot To Player`))
        (if (> _dot_left_right 0.0)
          (bind _returnvalue (`KismetMathLibrary.DegAtan2` _dot_left_right _dot_front_back))
          (set `local.TargetAngle` (+ _returnvalue (`local.RotationStep`)))
          (else
            (set `local.TargetAngle` (- _returnvalue (`local.RotationStep`)))))
        (`self.Event SetDestination` (+ (`Controller.GetPlayerViewPoint` (`GameplayStatics.GetPlayerController` 0)) (* (`KismetMathLibrary.Vector_Normal2D` (`KismetMathLibrary.RotateAngleAxis` (`KismetMathLibrary.GetForwardVector` (`.Rotation` (`Controller.GetPlayerViewPoint` (`GameplayStatics.GetPlayerController` 0)))) (`local.TargetAngle`) (`KismetMathLibrary.Vector_Up`))) (`self.distToPlayer`))))
        (return)))))

(fn `State Teleport`
  (if (not (`self.stateInitialized`))
    ;[1 1 1] Initialize State
    (set `self.stateInitialized` true)
    (set `self.hasTeleported` false))
  (if (`self.debugStates`)
    (`KismetSystemLibrary.PrintString` "TELEPORT"))
  (`|ExecutionSequence`
    (:`then_0`
      ;[1 1 1] Check for state changes
      (`|ExecutionSequence`
        (:`then_0`
          (if (`self.hasTeleported`)
            (`self.Event ChangeState` "NewEnumerator0")
            (return)))))
    (:`then_1`
      ;[1 1 1] Find random spot and teleport
      (`self.K2_SetActorLocation` (`NavigationSystemV1.K2_GetRandomReachablePointInRadius` (`self.K2_GetActorLocation`) 2000.0 null null) false true)
      (set `self.hasTeleported` true))))

(fn `UserConstructionScript`)